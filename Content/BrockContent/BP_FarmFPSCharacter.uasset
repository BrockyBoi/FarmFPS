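; Player character Blueprint for a farming FPS that displays the player's crop inventory and money on screen.
; On BeginPlay it creates the crop inventory and wallet widgets and adds both to the viewport.
; Each Tick it polls ResourceInventory for Wheat and Bread counts and PlayerWallet for money, pushing them into the widgets.
; The Bread update is nested under the wallet widget's validity check, so it depends on both widgets existing.
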(event `self.ReceiveBeginPlay`
  (bind _returnvalue (`|CreateWidget` "/Game/BrockContent/WBP_CropInventory.WBP_CropInventory_C"))
  (bind _output_get (set `self.InventoryWidget` _returnvalue))
  (`UserWidget.AddToViewport` _output_get 0)
  (bind _returnvalue_2 (`|CreateWidget` "/Game/BrockContent/WBP_PlayerWallet.WBP_PlayerWallet_C"))
  (bind _output_get_2 (set `self.PlayerWalletWidget` _returnvalue_2))
  (`UserWidget.AddToViewport` _output_get_2 0))

(event `self.ReceiveTick`
  (params (DeltaSeconds :type "Float (single-precision)"))
  (bind _resourceinventory (`self.ResourceInventory`))
  (bind _playerwalletwidget (`self.PlayerWalletWidget`))
  (bind _inventorywidget (`self.InventoryWidget`))
  (`/Engine/EditorBlueprintResources/StandardMacros.IsValid` _inventorywidget
    (:`Is Valid`
      (`/Game/BrockContent/WBP_CropInventory.SetCropYieldCount` _inventorywidget "Wheat" (`ResourceInventory.GetResourceCount` _resourceinventory "Wheat"))
      (`/Engine/EditorBlueprintResources/StandardMacros.IsValid` _playerwalletwidget
        (:`Is Valid`
          (`/Game/BrockContent/WBP_PlayerWallet.SetMoneyCount` _playerwalletwidget (`PlayerWallet.GetCurrentMoneyCount` (`self.PlayerWallet`)))
          (`/Game/BrockContent/WBP_CropInventory.SetCropYieldCount` _inventorywidget "Bread" (`ResourceInventory.GetResourceCount` _resourceinventory "Bread")))))))

(fn `UserConstructionScript`
  (`parent.UserConstructionScript`))