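; Game state Blueprint for the farm FPS that pushes objective progress to the player's HUD.
; It listens to ObjectiveManager events for progress updates, objective completion and main objective completion.
; Each calls SetObjectiveUIPercent, which casts the first player's pawn to BP_FarmFPSCharacter and sets its ObjectiveWidget progress to count over target.
; Both completion events pass a count of zero, resetting the displayed progress.
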(event `self.ObjectiveManager.OnObjectiveProgressUpdated`
  (params (objectiveData :type "ObjectiveData Structure") (newProgressCount :type Integer))
  (`self.SetObjectiveUIPercent` newProgressCount objectiveData))

(event `self.ObjectiveManager.OnObjectiveCompleted`
  (params (objectiveData :type "ObjectiveData Structure"))
  (`self.SetObjectiveUIPercent` 0 objectiveData))

(event `self.ObjectiveManager.OnMainObjectiveCompleted`
  (params (objectiveData :type "ObjectiveData Structure"))
  (`self.SetObjectiveUIPercent` 0 objectiveData))

(fn `SetObjectiveUIPercent`
  (params (`Progress Count` :type Integer) (`Objective Data` :type "ObjectiveData Structure"))
  (bind _asbp_farm_fpscharacter (cast `/Game/BrockContent/Characters/BP_FarmFPSCharacter` (`GameplayStatics.GetPlayerPawn` 0)))
  (bind _objectivewidget (`/Game/BrockContent/Characters/BP_FarmFPSCharacter.ObjectiveWidget` _asbp_farm_fpscharacter))
  (`/Engine/EditorBlueprintResources/StandardMacros.IsValid` _objectivewidget
    (:`Is Valid`
      (`/Game/BrockContent/UI/WBP_CurrentObjectiveProgressUI.SetObjectiveProgress` _objectivewidget (/ (`KismetMathLibrary.Conv_IntToDouble` `Progress Count`) (`KismetMathLibrary.Conv_IntToDouble` (`._objectiveProgressTarget` (break `ObjectiveData` `Objective Data`))))))))

(fn `UserConstructionScript`)