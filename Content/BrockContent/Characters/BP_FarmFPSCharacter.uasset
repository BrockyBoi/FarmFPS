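; First-person farm game character Blueprint that links its ResourceInventory to HUD widgets.
; Resource count changes send Money to the wallet widget and other types to the crop count widget, only when both widgets are valid.
; SetObjectiveProgress forwards a percentage to the objective widget, ignoring its Objective input.
; BeginPlay is empty; the logic creating these widgets and granting starter resources is disconnected and never runs.
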(event `self.ReceiveBeginPlay`)

(event `self.ResourceInventory.OnResourceCountChanged`
  (params (resourceType :type "GameplayTag Structure (by ref)") (newAmount :type "Float (single-precision)"))
  (bind _inventorywidget (`self.InventoryWidget`))
  (bind _playerwalletwidget (`self.PlayerWalletWidget`))
  (`/Engine/EditorBlueprintResources/StandardMacros.IsValid` _inventorywidget
    (:`Is Valid`
      (`/Engine/EditorBlueprintResources/StandardMacros.IsValid` _playerwalletwidget
        (:`Is Valid`
          (if (== resourceType (struct :`TagName` "ResourceType.Money"))
            (`/Game/BrockContent/UI/WBP_PlayerWallet.SetMoneyCount` _playerwalletwidget (`KismetMathLibrary.FTrunc` newAmount))
            (else
              (`/Game/BrockContent/UI/WBP_ResourceCounts.SetResourceCount` _inventorywidget resourceType (`KismetMathLibrary.FTrunc` newAmount)))))))))

(fn `SetObjectiveProgress`
  (params (Objective :type "ObjectiveData Structure") (ProgressPercent :type "Float (double-precision)"))
  (bind _objectivewidget (`self.ObjectiveWidget`))
  (`/Engine/EditorBlueprintResources/StandardMacros.IsValid` _objectivewidget
    (:`Is Valid`
      (`/Game/BrockContent/UI/WBP_CurrentObjectiveProgressUI.SetObjectiveProgress` _objectivewidget ProgressPercent))))

(fn `UserConstructionScript`
  (`parent.UserConstructionScript`))