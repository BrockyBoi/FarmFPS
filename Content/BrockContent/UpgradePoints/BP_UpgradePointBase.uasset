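; Base upgrade point Blueprint that presents a purchasable perk modifier upgrade and its cost.
; The construction script sets the Capsule as the overlapping component of UpgradePurchaceLocation, which holds the modifier tag and cost.
; Every Tick rebuilds the UpgradeDescription text from the tag name, stripped of its "PerkModifier." prefix, followed by the rounded cost.
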(event `self.ReceiveTick`
  (params (DeltaSeconds :type "Float (single-precision)"))
  (`TextRenderComponent.K2_SetText` (`self.Upgrade Description`) (`KismetTextLibrary.Conv_StringToText` (`KismetStringLibrary.Concat_StrStr` "" (`KismetStringLibrary.Replace` (`BlueprintGameplayTagLibrary.GetDebugStringFromGameplayTag` (`UpgradePurchaceLocation._modifierUpgrade` (`self.UpgradePurchaceLocation`))) "PerkModifier.") " $:" (`KismetStringLibrary.Conv_Int64ToString` (`KismetMathLibrary.Round64` (`UpgradePurchaceLocation._upgradeCost` (`self.UpgradePurchaceLocation`))))))))

(fn `UserConstructionScript`
  (set `UpgradePurchaceLocation._overlappingComponent` (`self.Capsule`) (`self.UpgradePurchaceLocation`)))