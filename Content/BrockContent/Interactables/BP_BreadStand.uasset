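; BP_BreadStand is an interactable stand that takes in bread, outputs money and has a customer queue.
; Its construction script assigns the bread input and money output colliders to their resource points and sets the queue's start location.
; Every Tick, it polls the input inventory for the bread gameplay tag and rewrites the count text as a whole number.
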(event `self.ReceiveTick`
  (params (DeltaSeconds :type "Float (single-precision)"))
  (`TextRenderComponent.K2_SetText` (`self.BreadCountText`) (`KismetTextLibrary.Conv_StringToText` (`KismetStringLibrary.Concat_StrStr` "Bread: " (`KismetStringLibrary.Conv_IntToString` (`KismetMathLibrary.FTrunc` (`ResourceInventory.GetResourceCount` (`self._inputInventory`) (`BlueprintGameplayTagLibrary.MakeLiteralGameplayTag` (struct :`TagName` "ResourceType.Bread")))))))))

(fn `UserConstructionScript`
  (set `AutomaticResourceTransferPoint._playerCollider` (`self.BreadInputCollider`) (`self._resourceInputPoint`))
  (set `AutomaticResourceTransferPoint._playerCollider` (`self.MoneyOutputCollider`) (`self._resourceOutputPoint`))
  (set `CustomerQueue._queueStartPoint` (`self.Queue Start Location`) (`self._customerQueue`)))