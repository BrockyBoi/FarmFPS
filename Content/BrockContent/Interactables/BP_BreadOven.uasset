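; BP_BreadOven is an interactable bread oven with resource input and output points and a widget that displays its crafting recipe.
; The construction script assigns the input and output colliders as the player colliders of their matching resource points.
; On BeginPlay, it zeroes the WBP_ResourceCounts widget, registers each required resource's tag and base amount from the CraftingRecipe, then destroys unused resource entries.
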(event `self.ReceiveBeginPlay`
  (bind _aswbp_resource_counts (cast `/Game/BrockContent/UI/WBP_ResourceCounts` (`WidgetComponent.GetWidget` (`self.RecipeWidget`))))
  (`/Game/BrockContent/UI/WBP_ResourceCounts.SetAllToZero` _aswbp_resource_counts)
  (for _array_element (`.RequiredResources` (break `CraftingData` (`self._craftingRecipe`)))
    (bind (_resourcetag _modifiedintvalue) (break `ModifiedResourceValue` _array_element))
    (`/Game/BrockContent/UI/WBP_ResourceCounts.AddAllowedResource` _aswbp_resource_counts _resourcetag)
    (`/Game/BrockContent/UI/WBP_ResourceCounts.SetResourceCount` _aswbp_resource_counts _resourcetag (`.BaseValue` (break `ModifiedIntValue` _modifiedintvalue))))
  (`/Game/BrockContent/UI/WBP_ResourceCounts.DestroyUnusedResources` _aswbp_resource_counts))

(fn `UserConstructionScript`
  (set `AutomaticResourceTransferPoint._playerCollider` (`self.InputCollider`) (`self._resourceInputPoint`))
  (set `AutomaticResourceTransferPoint._playerCollider` (`self.OutputCollider`) (`self._resourceOutputPoint`)))