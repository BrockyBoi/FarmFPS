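; Choppable tree in the plant-growth system that loses life per hit and falls once depleted.
; Each hit plays a material flash timeline, spawns dust and chop effects, and drops a random branch actor.
; At zero life it swaps to the after-harvest mesh and physics-simulates a separate trunk on NextMesh.
; A looping timer detects the trunk lying nearly horizontal, then after a delay hides it behind particle bursts along its length.
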(event `Destroy Trunk Delayed`
  (`/Engine/EditorBlueprintResources/StandardMacros.DoOnce` false
    (:`Completed`
      (`KismetSystemLibrary.Delay` 3.0)
      (`self.Destroy Trunk`))))

(event `self.ReceiveBeginPlay`
  (`parent.ReceiveBeginPlay`))

(event `self.ReceiveTick`
  (params (DeltaSeconds :type "Float (single-precision)"))
  (`parent.ReceiveTick` DeltaSeconds))

(event `/Game/DreamscapeSeries/SharedResources/Blueprints/Interfaces/BPI_Interaction.Trace Interactable Object`
  (params (HitResult :type "HitResult Structure")))

(event `/Game/DreamscapeSeries/SharedResources/Blueprints/Interfaces/BPI_Interaction.Interact`
  (params (`Hit Result` :type "HitResult Structure"))
  (bind (_bblockinghit _binitialoverlap _time _distance _location _impactpoint _normal _impactnormal _physmat _hitactor _hitcomponent _hitbonename _bonename _hititem _elementindex _faceindex _tracestart _traceend) (`GameplayStatics.BreakHitResult` `Hit Result`))
  (bind _returnvalue (`KismetMathLibrary.Normal` (- _traceend _tracestart)))
  (if (not (or (`TimelineComponent.IsPlaying` (`self.Hit Timeline`)) (`self.Chopped`)))
    (`TimelineComponent.PlayFromStart` (`self.Hit Timeline`))
    (`NiagaraFunctionLibrary.SpawnSystemAtLocation` "/Game/DreamscapeSeries/SharedResources/Particles/Niagara/NS_DustBurst.NS_DustBurst" (+ _tracestart (* _returnvalue (- _distance 15.0))))
    (`ActorComponent.Activate` (`self.NS_TreeChop`) true)
    (`/Engine/EditorBlueprintResources/StandardMacros.DecrementInt` (`self.Tree Life`)
      (:`  `
        (`self.Spawn Branch` _returnvalue)))))

(fn `Check Trunk Destruction`
  (bind _returnvalue (`SceneComponent.GetUpVector` (`self.Next Mesh`)))
  (if (> (`KismetMathLibrary.Dot_VectorVector` (`KismetMathLibrary.Normal` _returnvalue) (`KismetMathLibrary.Normal` (`KismetMathLibrary.ProjectVectorOnToPlane` _returnvalue (0.0 0.0 1.0)))) 0.9)
    (`KismetSystemLibrary.K2_ClearTimer` null "Check Trunk Destruction")
    (`self.Destroy Trunk Delayed`)))

(fn `Chop Tree`
  (set `self.Ready to Harvest` false)
  (`|ExecutionSequence`
    (:`then_0`
      (`PrimitiveComponent.SetCollisionEnabled` (`self.Capsule`) "NoCollision"))
    (:`then_1`
      (`StaticMeshComponent.SetStaticMesh` (`self.Current Mesh`) (`self.After Harvest Mesh`))
      (`PrimitiveComponent.SetCollisionEnabled` (`self.Current Mesh`) "QueryAndPhysics")
      (`self.Set Mesh Materials` (`self.Current Mesh`) (`self.After Harvest Mesh`)))
    (:`then_2`
      (`StaticMeshComponent.SetStaticMesh` (`self.Next Mesh`) (`self.Trunk Mesh`))
      (`SceneComponent.SetVisibility` (`self.Next Mesh`) true false)
      (`PrimitiveComponent.SetAngularDamping` (`self.Next Mesh`) 1.0)
      (`PrimitiveComponent.SetCollisionObjectType` (`self.Next Mesh`) "ECC_WorldDynamic")
      (`PrimitiveComponent.SetCollisionEnabled` (`self.Next Mesh`) "QueryAndPhysics")
      (`PrimitiveComponent.SetSimulatePhysics` (`self.Next Mesh`) true)
      (`self.Set Mesh Materials` (`self.Next Mesh`) (`self.Trunk Mesh`)))
    (:`then_3`
      (`KismetSystemLibrary.K2_SetTimer` null "Check Trunk Destruction" 0.1 true))))

(fn `Destroy Trunk`
  (locals (`Num Of Particles` :type Integer :default 0) (`Initial Offset` :type "Float (double-precision)" :default 0.0))
  (bind _next_mesh (`self.Next Mesh`))
  (bind (_min _max) (`StaticMeshComponent.GetLocalBounds` (`self.Next Mesh`)))
  (bind _z (.z _min))
  (`PrimitiveComponent.SetSimulatePhysics` (`self.Next Mesh`) false)
  (`PrimitiveComponent.SetCollisionResponseToAllChannels` (`self.Next Mesh`) "ECR_Ignore")
  (`PrimitiveComponent.SetCollisionEnabled` (`self.Next Mesh`) "NoCollision")
  (`SceneComponent.SetVisibility` (`self.Next Mesh`) false false)
  (set `local.Initial Offset` _z)
  (set `local.Num Of Particles` (`KismetMathLibrary.FFloor` (* (/ (`KismetMathLibrary.Abs` (- _z (.z _max))) 150.0) 0.6)))
  (for _index (range (+ (`local.Num Of Particles`) 1))
    (`NiagaraFunctionLibrary.SpawnSystemAtLocation` "/Game/DreamscapeSeries/SharedResources/Particles/Niagara/NS_FoliageHarvest.NS_FoliageHarvest" (+ (`SceneComponent.K2_GetComponentLocation` _next_mesh) (* (`SceneComponent.GetUpVector` _next_mesh) (+ (* _index 150) (`local.Initial Offset`)))))))

(fn `Set Up Harvesting`
  (`parent.Set Up Harvesting`)
  (`self.Set Static Mesh By Stage Index` (`KismetArrayLibrary.Array_LastIndex` (`self.Plant Stages`)) (`self.Current Mesh`) (`self.Current Materials`))
  (`PrimitiveComponent.SetCollisionResponseToChannel` (`self.Current Mesh`) "ECC_GameTraceChannel1" "ECR_Block"))

(fn `Set Up Interaction Capsule`)

(fn `Setup NextMesh on Grown`
  (`StaticMeshComponent.SetStaticMesh` (`self.Next Mesh`) null)
  (`SceneComponent.SetVisibility` (`self.Next Mesh`) false false))

(fn `Spawn Branch`
  (params (`Facing Direction` :type "Vector Structure"))
  (locals (`Center Location` :type "Vector Structure" :default (0.0 0.0 0.0)) (`Branch Direction Vector` :type "Vector Structure" :default (0.0 0.0 0.0)))
  (set `local.Center Location` (`SceneComponent.K2_GetComponentLocation` (`self.NS_TreeChop`)))
  (set `local.Branch Direction Vector` (`KismetMathLibrary.Normal` (`KismetMathLibrary.MakeVector` (.x (`local.Facing Direction`)) (.y (`local.Facing Direction`)))))
  (`|SpawnActorFromClass` (`KismetArrayLibrary.Array_Random` (`self.Falling Branch Meshes`)) (`KismetMathLibrary.MakeTransform` (`KismetMathLibrary.MakeVector` (.x (+ (`local.Center Location`) (* (`local.Branch Direction Vector`) (`KismetMathLibrary.RandomFloatInRange` 400.0 550.0)))) (.y (+ (`local.Center Location`) (* (`local.Branch Direction Vector`) (`KismetMathLibrary.RandomFloatInRange` 400.0 550.0)))) (+ (.z (`local.Center Location`)) 150.0)) (`KismetMathLibrary.FindLookAtRotation` (`local.Center Location`) (+ (`local.Center Location`) (`KismetMathLibrary.RotateAngleAxis` (`local.Branch Direction Vector`) (`KismetMathLibrary.RandomFloatInRange` -120.0 120.0) (0.0 0.0 1.0)) (0.0 0.0 0.35)))) "Undefined" "SelectDefaultAtRuntime" self null))

(fn `UserConstructionScript`)