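; Growable plant actor that advances through timed PlantStages and becomes harvestable at the last one.
; Each stage change plays a timeline that crossfades two mesh components via a "Grow Animation" material parameter, then swaps them.
; When grown, it fits a trace-blocking capsule to mesh bounds; traces reveal an outline mesh and text, which Tick hides again.
; Interact spawns harvest Niagara, disables collision, and shows AfterHarvestMesh or hides the plant.
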(event `self.ReceiveBeginPlay`
  (set `self.Current Stage` 0)
  (`self.Check Final Stage`
    (:`Not Final`
      (`self.Set Static Mesh By Stage Index` 0 (`self.Next Mesh`) (`self.Next Materials`))
      (`KismetSystemLibrary.K2_SetTimer` null "Grow" (`.StageDurationsec_11_7CAD989D4A5633B88D5D71AECBF7F8B8` (break `/Game/DreamscapeSeries/SharedResources/Blueprints/PlantGrowth/Structs/F_PlantGrowthStageNew` (`|GetArrayItem` (`self.Plant Stages`) (`self.Current Stage`))))))))

(event `self.ReceiveTick`
  (params (DeltaSeconds :type "Float (single-precision)"))
  (if (`self.Ready to Harvest`)
    (`SceneComponent.SetVisibility` (`self.TextRender`) false false)
    (`SceneComponent.SetVisibility` (`self.Next Mesh`) false false)))

(event `Grow`
  (bind _returnvalue (+ (`self.Current Stage`) 1))
  (if (`KismetArrayLibrary.Array_IsValidIndex` (`self.Plant Stages`) _returnvalue)
    (set `self.Current Stage` _returnvalue)
    (`self.Set Static Mesh By Stage Index` (`self.Current Stage`) (`self.Next Mesh`) (`self.Next Materials`))
    (`TimelineComponent.PlayFromStart` (`self.Transition Timeline`))))

(event `/Game/DreamscapeSeries/SharedResources/Blueprints/Interfaces/BPI_Interaction.Trace Interactable Object`
  (params (HitResult :type "HitResult Structure"))
  (bind (_bblockinghit _binitialoverlap _time _distance _location _impactpoint _normal _impactnormal _physmat _hitactor _hitcomponent _hitbonename _bonename _hititem _elementindex _faceindex _tracestart _traceend) (`GameplayStatics.BreakHitResult` HitResult))
  (if (`self.Ready to Harvest`)
    (`SceneComponent.SetVisibility` (`self.Next Mesh`) true false)
    (`SceneComponent.K2_SetWorldRotation` (`self.TextRender`) (`KismetMathLibrary.Conv_VectorToRotator` (`KismetMathLibrary.Normal` (- _tracestart _traceend))) false false)
    (`SceneComponent.SetVisibility` (`self.TextRender`) true false)))

(event `/Game/DreamscapeSeries/SharedResources/Blueprints/Interfaces/BPI_Interaction.Interact`
  (params (`Hit Result` :type "HitResult Structure"))
  (set `self.Ready to Harvest` false)
  (`PrimitiveComponent.SetCollisionEnabled` (`self.Current Mesh`) "NoCollision")
  (`PrimitiveComponent.SetCollisionEnabled` (`self.Next Mesh`) "NoCollision")
  (`PrimitiveComponent.SetCollisionEnabled` (`self.Capsule`) "NoCollision")
  (`SceneComponent.SetVisibility` (`self.TextRender`) false false)
  (`NiagaraFunctionLibrary.SpawnSystemAttached` "/Game/DreamscapeSeries/SharedResources/Particles/Niagara/NS_FoliageHarvest.NS_FoliageHarvest" (`self.DefaultSceneRoot`) "None" (0.0 0.0 0.0) (struct) "KeepRelativeOffset" true)
  (`SceneComponent.SetVisibility` (`self.Next Mesh`) false false)
  (`/Engine/EditorBlueprintResources/StandardMacros.IsValid` (`self.After Harvest Mesh`)
    (:`Is Valid`
      (`StaticMeshComponent.SetStaticMesh` (`self.Current Mesh`) (`self.After Harvest Mesh`)))
    (:`Is Not Valid`
      (`SceneComponent.SetVisibility` (`self.Current Mesh`) false false))))

(fn `Set Static Mesh By Stage Index`
  (params (Index :type Integer) (`In Comp` :type "StaticMeshComponent Object Reference") (Materials :type "Array of MaterialInstanceDynamic Object Reference (by ref)"))
  (bind _plantmesh (break `/Game/DreamscapeSeries/SharedResources/Blueprints/PlantGrowth/Structs/F_PlantGrowthStageNew` (`|GetArrayItem` (`self.Plant Stages`) Index)))
  (`/Engine/EditorBlueprintResources/StandardMacros.IsValid` _plantmesh
    (:`Is Valid`
      (`KismetArrayLibrary.Array_Clear` (`local.Materials`))
      (`StaticMeshComponent.SetStaticMesh` `In Comp` _plantmesh)
      (for (_array_element _array_index) (`StaticMesh.StaticMaterials` _plantmesh)
        (bind _returnvalue (`KismetMaterialLibrary.CreateDynamicMaterialInstance` (`.MaterialInterface` (break `StaticMaterial` _array_element))))
        (`PrimitiveComponent.SetMaterial` (`local.In Comp`) _array_index _returnvalue)
        (`KismetArrayLibrary.Array_Add` (`local.Materials`) _returnvalue)))))

(fn `Set Up Harvesting`
  (bind _plant_stages (`self.Plant Stages`))
  (set `self.Ready to Harvest` true)
  (`StaticMeshComponent.SetStaticMesh` (`self.Current Mesh`) (`.PlantMesh_2_7F6EADE74110AFEFBE837D893570C28C` (break `/Game/DreamscapeSeries/SharedResources/Blueprints/PlantGrowth/Structs/F_PlantGrowthStageNew` (`|GetArrayItem` _plant_stages (`KismetArrayLibrary.Array_LastIndex` _plant_stages)))))
  (`self.Setup NextMesh on Grown`)
  (`self.Set Up Interaction Capsule`))

(fn `Set Up Interaction Capsule`
  (locals (`Capsule Position` :type "Vector Structure") (`Local Bounds Differences` :type "Vector Structure") (MaxX :type Boolean) (MaxY :type Boolean))
  (bind _current_mesh (`self.Current Mesh`))
  (bind _capsule (`self.Capsule`))
  (bind (_local_bounds_differences_x _local_bounds_differences_y _local_bounds_differences_z) (`KismetMathLibrary.BreakVector` (`local.Local Bounds Differences`)))
  (bind (_local_bounds_differences_x_2 _local_bounds_differences_y_2 _local_bounds_differences_z_2) (`KismetMathLibrary.BreakVector` (`local.Local Bounds Differences`)))
  (bind (_local_bounds_differences_x_3 _local_bounds_differences_y_3 _local_bounds_differences_z_3) (`KismetMathLibrary.BreakVector` (`local.Local Bounds Differences`)))
  (bind (_origin _boxextent) (`KismetSystemLibrary.GetComponentBounds` _current_mesh))
  (bind _x (.x (`local.Local Bounds Differences`)))
  (bind _y (.y (`local.Local Bounds Differences`)))
  (bind _z (.z (`local.Local Bounds Differences`)))
  (set `local.Capsule Position` (`KismetMathLibrary.InverseTransformLocation` (`SceneComponent.K2_GetComponentToWorld` _current_mesh) _origin))
  (set `local.Local Bounds Differences` _boxextent)
  (set `local.MaxX` (and (>= _x _y) (>= _x _z)))
  (set `local.MaxY` (and (>= _y _x) (>= _y _z)))
  (set `self.Mesh Radius` (`KismetMathLibrary.SelectFloat` (`KismetMathLibrary.FMax` _local_bounds_differences_y_3 _local_bounds_differences_z_3) (`KismetMathLibrary.SelectFloat` (`KismetMathLibrary.FMax` _local_bounds_differences_x_3 _local_bounds_differences_z_3) (`KismetMathLibrary.FMax` _local_bounds_differences_x_3 _local_bounds_differences_y_3) (`local.MaxY`)) (`local.MaxX`)))
  (`SceneComponent.K2_AddLocalRotation` (`self.Capsule`) (`KismetMathLibrary.SelectRotator` (struct :`Pitch` 90.0) (`KismetMathLibrary.SelectRotator` (struct :`Roll` 90.0) (struct) (`local.MaxY`)) (`local.MaxX`)) false false)
  (`CapsuleComponent.SetCapsuleHalfHeight` (`self.Capsule`) (+ (`KismetMathLibrary.SelectFloat` _local_bounds_differences_x (`KismetMathLibrary.SelectFloat` _local_bounds_differences_y _local_bounds_differences_z (`local.MaxY`)) (`local.MaxX`)) (/ (`self.Mesh Radius`) 2.0)) true)
  (`SceneComponent.K2_SetRelativeLocation` (`self.Capsule`) (`local.Capsule Position`) false false)
  (`CapsuleComponent.SetCapsuleRadius` (`self.Capsule`) (`self.Mesh Radius`) true)
  (`SceneComponent.K2_SetWorldLocation` (`self.TextRender`) (+ (`SceneComponent.K2_GetComponentLocation` (`self.Capsule`)) (`KismetMathLibrary.MakeVector` 0.0 0.0 _local_bounds_differences_z_2) (0.0 0.0 20.0)) false false)
  (`PrimitiveComponent.SetCollisionResponseToAllChannels` _capsule "ECR_Ignore")
  (`PrimitiveComponent.SetCollisionResponseToChannel` _capsule "ECC_GameTraceChannel1" "ECR_Block"))

(fn `Setup NextMesh on Grown`
  (bind _plant_stages (`self.Plant Stages`))
  (`StaticMeshComponent.SetStaticMesh` (`self.Next Mesh`) (`.PlantMesh_2_7F6EADE74110AFEFBE837D893570C28C` (break `/Game/DreamscapeSeries/SharedResources/Blueprints/PlantGrowth/Structs/F_PlantGrowthStageNew` (`|GetArrayItem` _plant_stages (`KismetArrayLibrary.Array_LastIndex` _plant_stages)))))
  (`PrimitiveComponent.SetMaterialByName` (`self.Next Mesh`) "CropSlot" "/Game/DreamscapeSeries/SharedResources/MasterMaterials/BaseMaterials/M_Outline.M_Outline"))

(fn `Swap Meshes`
  (locals (`Temp Comp` :type "StaticMeshComponent Object Reference") (`Temp Materials` :type "Array of MaterialInstanceDynamic Object Reference"))
  (set `local.Temp Comp` (`self.Current Mesh`))
  (set `self.Current Mesh` (`self.Next Mesh`))
  (set `self.Next Mesh` (`local.Temp Comp`))
  (set `local.Temp Materials` (`self.Current Materials`))
  (set `self.Current Materials` (`self.Next Materials`))
  (set `self.Next Materials` (`local.Temp Materials`)))

(fn `UserConstructionScript`
  (`self.Set Static Mesh By Stage Index` (`KismetArrayLibrary.Array_LastIndex` (`self.Plant Stages`)) (`self.Next Mesh`) (`self.Next Materials`)))