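; Falling branch actor for the plant growth system that breaks apart shortly after landing.
; BoxCollision carries the physics while the mesh has no collision; Tick derives acceleration from velocity change and treats the first upward value as impact.
; After a delay it hides the mesh and spawns foliage Niagara bursts evenly along the box's longest axis.
; The actor-destroy handler's binding never runs, so the hidden actor remains.
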(event `self.ReceiveTick`
  (params (DeltaSeconds :type "Float (single-precision)"))
  (bind _returnvalue (`PrimitiveComponent.GetPhysicsLinearVelocity` (`self.Box Collision`) "None"))
  (set `self.Acceleration` (/ (- _returnvalue (`self.Prev Velocity`)) DeltaSeconds))
  (set `self.Prev Velocity` _returnvalue)
  (if (> (.z (`self.Acceleration`)) 0.0)
    (`/Engine/EditorBlueprintResources/StandardMacros.DoOnce` false
      (:`Completed`
        (`KismetSystemLibrary.Delay` 2.0)
        (`SceneComponent.SetVisibility` (`self.Branch Mesh`) false false)
        (`self.Spawn Break Particles`)))))

(event `OnSystemFinished_Event`
  (params (PSystem :type "NiagaraComponent Object Reference"))
  (`self.K2_DestroyActor`))

(fn `Calculate Particle Spawn Points`
  (returns (`Orientation Axis` :type "ESplineMeshAxis Enum"))
  (bind _x (.x (`BoxComponent.GetScaledBoxExtent` (`self.Box Collision`))))
  (bind _y (.y (`BoxComponent.GetScaledBoxExtent` (`self.Box Collision`))))
  (bind _z (.z (`BoxComponent.GetScaledBoxExtent` (`self.Box Collision`))))
  (if (> _x _y)
    (if (> _x _z)
      (return "X")
      (else
        (return "Z")))
    (elif (> _y _z)
      (return "Y")
      (else
        (return "Z")))))

(fn `Spawn Break Particles`
  (locals (`Orientation Axis` :type "ESplineMeshAxis Enum" :default "X") (`Box Half Length` :type "Float (double-precision)") (`Num of Particles` :type Integer :default 0))
  (bind _box_collision (`self.Box Collision`))
  (bind (_returnvalue_x _returnvalue_y _returnvalue_z) (`KismetMathLibrary.BreakVector` (`BoxComponent.GetScaledBoxExtent` (`self.Box Collision`))))
  (bind _returnvalue (`SceneComponent.K2_GetComponentLocation` (`self.Box Collision`)))
  (bind _returnvalue_2 (* (select `ESplineMeshAxis` (`local.Orientation Axis`) :`X` (`SceneComponent.GetForwardVector` _box_collision) :`Y` (`SceneComponent.GetRightVector` _box_collision) :`Z` (`SceneComponent.GetUpVector` _box_collision)) (`local.Box Half Length`)))
  (bind _orientation_axis (`self.Calculate Particle Spawn Points`))
  (set `local.Orientation Axis` _orientation_axis)
  (bind _output_get (set `local.Box Half Length` (select `ESplineMeshAxis` (`local.Orientation Axis`) :`X` _returnvalue_x :`Y` _returnvalue_y :`Z` _returnvalue_z)))
  (set `local.Num of Particles` (`KismetMathLibrary.FFloor` (/ (* _output_get 2.0) 150.0)))
  (for _index (range (+ (`local.Num of Particles`) 1))
    (`NiagaraFunctionLibrary.SpawnSystemAtLocation` "/Game/DreamscapeSeries/SharedResources/Particles/Niagara/NS_FoliageHarvest.NS_FoliageHarvest" (`KismetMathLibrary.VLerp` (+ _returnvalue _returnvalue_2) (- _returnvalue _returnvalue_2) (/ _index (`local.Num of Particles`))))))

(fn `UserConstructionScript`
  (`PrimitiveComponent.SetCollisionEnabled` (`self.Branch Mesh`) "NoCollision"))